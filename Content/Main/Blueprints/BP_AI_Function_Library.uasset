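; Blueprint function library of helpers for grid squares, tagged-actor lookup and cursor targeting.
; Two functions toggle BP_Grid_Square box collision: reset disables it on every square, set enables it on occupied ones.
; RetrieveClickedTargetInfo traces under the first player's cursor and reports whether the hit actor derives from a given class.
; CastToActorWithTag searches actors of a class for a tag, but returns after checking only the first element.
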(fn `CastToActorWithTag`
  (params (Actor :type "Actor Class Reference") (Tag :type Name))
  (returns (foundActor :type Boolean) (foundActorRef :type "Actor Object Reference"))
  (bind _outactors (`GameplayStatics.GetAllActorsOfClass` null Actor))
  (for _array_element _outactors
    (if (`Actor.ActorHasTag` _array_element Tag)
      (return true _array_element)
      (else
        (return false _array_element)))))

(fn `ResetAllOccupiedSpaces`
  (bind _outactors (`GameplayStatics.GetAllActorsOfClass` null "/Game/Main/Blueprints/BP_Grid_Square.BP_Grid_Square_C"))
  (for _array_element _outactors
    (`PrimitiveComponent.SetCollisionEnabled` (`/Game/Main/Blueprints/BP_Grid_Square.Box` _array_element) "NoCollision")))

(fn `RetrieveClickedTargetInfo`
  (params (`Class to check for` :type "Actor Class Reference"))
  (returns (`Was Found` :type Boolean) (`Actor Clicked` :type "Actor Object Reference"))
  (bind (_bblockinghit _binitialoverlap _time _location _impactpoint _normal _impactnormal _physmat _hitactor) (`GameplayStatics.BreakHitResult` (`PlayerController.GetHitResultUnderCursorForObjects` (`GameplayStatics.GetPlayerController` null) (`|MakeArray` "ObjectTypeQuery3" "ObjectTypeQuery1" "ObjectTypeQuery2" :!type "EObjectTypeQuery Enum") true)))
  (if (`KismetMathLibrary.ClassIsChildOf` (`GameplayStatics.GetObjectClass` _hitactor) `Class to check for`)
    (return true _hitactor)
    (else
      (return false _hitactor))))

(fn `SetAllOccupiedSpaces`
  (bind _outactors (`GameplayStatics.GetAllActorsOfClass` null "/Game/Main/Blueprints/BP_Grid_Square.BP_Grid_Square_C"))
  (for _array_element _outactors
    (if (`/Game/Main/Blueprints/BP_Grid_Square.isOccupied` _array_element)
      (`PrimitiveComponent.SetCollisionEnabled` (`/Game/Main/Blueprints/BP_Grid_Square.Box` _array_element) "QueryAndPhysics")))
  (return))