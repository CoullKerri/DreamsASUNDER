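; Player camera that the top-down controller possesses on BeginPlay, providing screen panning and hero selection.
; It creates the BP_Camera_Panning widget, focuses it with the mouse locked to the viewport, and passes it a self-reference and the panning amount.
; Left-clicking a BP_Hero_Character turns its mesh yellow, sets it as the BP_Game_HUD's selected actor and prints its name.
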(event `self.ReceiveBeginPlay`
  (`|ExecutionSequence`
    (:`then_0`
      ;[1 1 1] Make the BP_Player_Camera the main camera
      (bind _astop_down_controller (cast `/Game/Main/Blueprints/TopDownController` (`GameplayStatics.GetPlayerController` 0)))
      (`Controller.Possess` _astop_down_controller self))
    (:`then_1`
      ;[1 1 1] Create the screen panning widget
      (bind _returnvalue (`|CreateWidget` "/Game/Main/Blueprints/BP_Camera_Panning.BP_Camera_Panning_C"))
      (bind _output_get (set `self.PanningWidget` _returnvalue))
      (`UserWidget.AddToViewport` _output_get 0)
      (`WidgetBlueprintLibrary.SetInputMode_GameAndUIEx` null _output_get true))
    (:`then_2`
      ;[1 1 1] Give the panning widget this blueprints id
      (set `/Game/Main/Blueprints/BP_Camera_Panning.playerCameraRef` self (`self.PanningWidget`))
      ;[1 1 1] Set the panning amount
      (set `/Game/Main/Blueprints/BP_Camera_Panning.panningAmount` (`self.panningAmount`) (`self.PanningWidget`)))))

(event `self.ReceiveActorBeginOverlap`
  (params (OtherActor :type "Actor Object Reference")))

(event `self.ReceiveTick`
  (params (DeltaSeconds :type "Float (single-precision)")))

(event `InputAction|LeftMouseButton` :consume false
  (params (Key :type "Key Structure" :default "AnyKey"))
  (:`Pressed`
    (bind (_was_found _actor_clicked) (`/Game/Main/Blueprints/BP_AI_Function_Library.RetrieveClickedTargetInfo` "/Game/Main/Blueprints/Characters/BP_Hero_Character.BP_Hero_Character_C"))
    (if _was_found
      (bind _asbp_hero_character (cast `/Game/Main/Blueprints/Characters/BP_Hero_Character` _actor_clicked))
      (`PrimitiveComponent.SetMaterial` (`Character.Mesh` _asbp_hero_character) 0 "/Game/Main/Textures_Materials/Yellow_MAT.Yellow_MAT")
      (bind _foundwidgets (`WidgetBlueprintLibrary.GetAllWidgetsOfClass` "/Game/Main/Blueprints/Widgets/BP_Game_HUD.BP_Game_HUD_C"))
      (bind _asbp_game_hud (cast `/Game/Main/Blueprints/Widgets/BP_Game_HUD` (`KismetArrayLibrary.Array_Get` _foundwidgets)))
      (set `/Game/Main/Blueprints/Widgets/BP_Game_HUD.selectedActor` _actor_clicked _asbp_game_hud)
      (`KismetSystemLibrary.PrintString` (`KismetSystemLibrary.GetDisplayName` _actor_clicked)))))

(fn `UserConstructionScript`)