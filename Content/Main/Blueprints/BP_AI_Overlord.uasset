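; Overlord actor for click-to-move on a grid: takes player input and finds the tagged character, with path building unfinished.
; Left-click highlights the BP_Grid_Square under the cursor, then CreateMovementPath measures X/Y offsets in 150-unit steps.
; It line-traces square to square along X only and never moves the character, so its outer loop has no exit.
; P runs DistanceCheck, intended to highlight squares along a short forward +X trace.
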(event `InputAction|LeftMouseButton`
  (params (Key :type "Key Structure" :default "AnyKey"))
  ;[1 1 1] Click and go there
)

(event `self.ReceiveBeginPlay`
  (bind _returnvalue (`self.CastToPlayerController` (`GameplayStatics.GetPlayerController` 0)))
  (`self.EnableInput` _returnvalue)
  (bind (_foundactor _foundactorref) (`/Game/Main/Blueprints/BP_AI_Function_Library.CastToActorWithTag` "/Game/Main/Blueprints/TopDownCharacter.TopDownCharacter_C" (`self.myCharacterTag`)))
  (if _foundactor
    (set `self.myCharRef` _foundactorref)))

(event `self.ReceiveTick`
  (params (DeltaSeconds :type "Float (single-precision)"))
  (set `self.DeltaTime` DeltaSeconds))

(event `Key|P`
  (params (Key :type "Key Structure" :default "AnyKey"))
  (:`Pressed`
    (`self.DistanceCheck`)))

(event `InputAction|LeftMouseButton`
  (params (Key :type "Key Structure" :default "AnyKey"))
  (:`Pressed`
    (bind (_was_found _actorclicked) (`self.RetrieveClickTargetInfo` "/Game/Main/Blueprints/BP_Grid_Square.BP_Grid_Square_C"))
    (if _was_found
      (bind _output_get (set `self.clickedActorRef` _actorclicked))
      (bind _asbp_grid_square (cast `/Game/Main/Blueprints/BP_Grid_Square` _output_get))
      (`PaperSpriteComponent.SetSprite` (`/Game/Main/Blueprints/BP_Grid_Square.Sprite` _asbp_grid_square) "/Game/Main/Sprites/Grid_Box_Hover_Sprite.Grid_Box_Hover_Sprite")
      (`self.CreateMovementPath`))))

(fn `CreateMovementPath`
  (bind _x (.x (`self.K2_GetActorLocation` (`self.myCharRef`))))
  (bind _x_2 (.x (`self.K2_GetActorLocation` (`self.clickedActorRef`))))
  (bind _y (.y (`self.K2_GetActorLocation` (`self.myCharRef`))))
  (bind _y_2 (.y (`self.K2_GetActorLocation` (`self.clickedActorRef`))))
  (`|ExecutionSequence`
    (:`then_0`
      (`/Engine/EditorBlueprintResources/StandardMacros.CompareFloat` _x _x_2
        (:`>`
          (while (!= (- _x _x_2) (`self.xDiff`))
            (set `self.xDiff` (+ (`self.xDiff`) 150.0))))
        (:`<`
          (while (!= (- _x_2 _x) (`self.xDiff`))
            (set `self.xDiff` (+ (`self.xDiff`) 150.0))))))
    (:`then_1`
      (`/Engine/EditorBlueprintResources/StandardMacros.CompareFloat` _y _y_2
        (:`>`
          (while (!= (- _y _y_2) (`self.yDiff`))
            (set `self.yDiff` (+ (`self.yDiff`) 150.0))))
        (:`<`
          (while (!= (- _y_2 _y) (`self.yDiff`))
            (set `self.yDiff` (+ (`self.yDiff`) 150.0))))))
    (:`then_2`
      (`|ExecutionSequence`
        (:`then_0`
          (if (not (< (.x (`self.K2_GetActorLocation` (`self.myCharRef`))) (.x (`self.K2_GetActorLocation` (`self.clickedActorRef`)))))
            (set `self.xSubAmount` (* (`self.xSubAmount`) -1.0))))
        (:`then_1`
          (if (not (< (.y (`self.K2_GetActorLocation` (`self.myCharRef`))) (.y (`self.K2_GetActorLocation` (`self.clickedActorRef`)))))
            (set `self.ySubAmount` (* (`self.ySubAmount`) -1.0))))
        (:`then_2`
          (set `self.currentPathGridLocation` (`self.K2_GetActorLocation` (`self.myCharRef`))))))
    (:`then_3`
      (while (!= (.x (`self.K2_GetActorLocation` (`self.myCharRef`))) (.x (`self.K2_GetActorLocation` (`self.clickedActorRef`))))
        (while (and (!= (`self.xObstructed`) true) (!= (`self.xDiff`) 0.0))
          (bind _outhit (`KismetSystemLibrary.LineTraceSingleForObjects` (`self.currentPathGridLocation`) (`KismetMathLibrary.MakeVector` (+ (.x (`self.currentPathGridLocation`)) (`self.xSubAmount`)) (.y (`self.currentPathGridLocation`)) (.z (`self.currentPathGridLocation`))) (`|MakeArray` "ObjectTypeQuery2" :!type "EObjectTypeQuery Enum")))
          (set `self.currentPathGridLocation` (`self.K2_GetActorLocation` (`.HitActor` (`GameplayStatics.BreakHitResult` _outhit))))
          (set `self.xDiff` (- (`self.xDiff`) 150.0)))))))

(fn `DistanceCheck`
  (`|ExecutionSequence`
    (:`then_0`
      (if true
        (bind _outhits (`KismetSystemLibrary.LineTraceMultiForObjects` (`KismetMathLibrary.MakeVector` (.x (`self.K2_GetActorLocation`)) (.y (`self.K2_GetActorLocation`)) 85.0) (`KismetMathLibrary.MakeVector` (+ (.x (`self.K2_GetActorLocation`)) 300.0) (.y (`self.K2_GetActorLocation`)) 85.0) (`|MakeArray` "ObjectTypeQuery2" :!type "EObjectTypeQuery Enum")))
        (for _array_element _outhits
          (bind (_bblockinghit _binitialoverlap _time _location _impactpoint _normal _impactnormal _physmat _hitactor) (`GameplayStatics.BreakHitResult` _array_element))
          (if (not (== _hitactor "/Game/Main/Blueprints/BP_Grid_Square.BP_Grid_Square_C"))
            (bind _asbp_grid_square (cast `/Game/Main/Blueprints/BP_Grid_Square` _hitactor))
            (`PaperSpriteComponent.SetSprite` (`/Game/Main/Blueprints/BP_Grid_Square.Sprite` _asbp_grid_square) "/Game/Main/Sprites/Grid_Box_Hover_Sprite.Grid_Box_Hover_Sprite")
            (`KismetSystemLibrary.PrintString` "Hello")))))))

(fn `RetrieveClickTargetInfo`
  (params (ClassToCheckFor :type "Actor Class Reference"))
  (returns (`Was Found` :type Boolean) (ActorClicked :type "Actor Object Reference"))
  (bind _returnvalue (`self.CastToPlayerController` (`GameplayStatics.GetPlayerController` 0)))
  (bind (_bblockinghit _binitialoverlap _time _location _impactpoint _normal _impactnormal _physmat _hitactor) (`GameplayStatics.BreakHitResult` (`PlayerController.GetHitResultUnderCursorForObjects` _returnvalue (`|MakeArray` "ObjectTypeQuery2" :!type "EObjectTypeQuery Enum") true)))
  (if (`KismetMathLibrary.ClassIsChildOf` (`GameplayStatics.GetObjectClass` _hitactor) ClassToCheckFor)
    (return true _hitactor)
    (else
      (return false _hitactor))))

(fn `UserConstructionScript`)