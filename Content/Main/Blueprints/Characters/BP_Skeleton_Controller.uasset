(event `self.ReceiveBeginPlay`
  (`|ExecutionSequence`
    (:`then_0`
      ;[1 1 1] Create Game Hud Ref
      (bind _foundwidgets (`WidgetBlueprintLibrary.GetAllWidgetsOfClass` "/Game/Main/Blueprints/Widgets/BP_Game_HUD.BP_Game_HUD_C"))
      (bind _asbp_game_hud (cast `/Game/Main/Blueprints/Widgets/BP_Game_HUD` (`KismetArrayLibrary.Array_Get` _foundwidgets)))
      (set `self.gameHudRef` _asbp_game_hud))
    (:`then_1`
      ;[1 1 1] Create reference to player camera
      (bind _outactors (`GameplayStatics.GetAllActorsOfClass` "/Game/Main/Blueprints/BP_Player_Camera.BP_Player_Camera_C"))
      (set `self.playerCamera` (`KismetArrayLibrary.Array_Get` _outactors)))))

(event `Initiate Move`
  (bind _gamehudref (`self.gameHudRef`))
  (bind _gamehudref_2 (`self.gameHudRef`))
  ;[1 1 1] Initiate the move
  (bind _outactors (`GameplayStatics.GetAllActorsOfClass` "/Game/Main/Blueprints/Characters/BP_Hero_Character.BP_Hero_Character_C"))
  (bind _item (`KismetArrayLibrary.Array_Get` _outactors))
  (if (<= (`self.GetDistanceTo` (`self.myCharRef`) _item) 200.0)
    ;[1 1 1] If already in range, attack
    (set `/Game/Main/Blueprints/Widgets/BP_Game_HUD.attackerRef` (`self.myCharRef`) (`self.gameHudRef`))
    (set `/Game/Main/Blueprints/Widgets/BP_Game_HUD.victimRef` _item _gamehudref_2)
    (if (not (`self.hasAttacked`))
      (`/Game/Main/Blueprints/Widgets/BP_Game_HUD.Attack ` _gamehudref_2)
      (set `self.hasAttacked` true))
    (set `/Game/Main/Blueprints/Widgets/BP_Game_HUD.currentEnemyIndex` (+ (`/Game/Main/Blueprints/Widgets/BP_Game_HUD.currentEnemyIndex` _gamehudref) 1) _gamehudref)
    (`/Game/Main/Blueprints/Widgets/BP_Game_HUD.Perform Skeleton Actions` (`self.gameHudRef`))
    (else
      (bind _outactors_2 (`GameplayStatics.GetAllActorsOfClass` "/Game/Main/Blueprints/Characters/BP_Hero_Character.BP_Hero_Character_C"))
      (`self.MoveToLocation` (`self.K2_GetActorLocation` (`KismetArrayLibrary.Array_Get` _outactors_2)) -1.0 false true false false))))

(event `self.ReceiveTick`
  (params (DeltaSeconds :type "Float (single-precision)"))
  ;[1 1 1] TEMP - Setting health text render to face camera
  (bind _asbp_skeleton_character (cast `/Game/Main/Blueprints/Characters/BP_Skeleton_Character` (`self.myCharRef`)))
  (bind _healthtext (`/Game/Main/Blueprints/Characters/BP_Skeleton_Character.HealthText` _asbp_skeleton_character))
  (`SceneComponent.K2_SetWorldRotation` _healthtext (.rotation (`self.GetTransform` (`self.playerCamera`))) false false)
  (`SceneComponent.K2_AddLocalRotation` _healthtext (struct :`Pitch` 45.0 :`Yaw` 180.0) false false)
  ;[1 1 1] Set Health
  (`TextRenderComponent.K2_SetText` _healthtext (`KismetTextLibrary.Conv_IntToText` (`self.myHealth`))))

(event `End Move`
  (bind _gamehudref (`self.gameHudRef`))
  (bind _gamehudref_2 (`self.gameHudRef`))
  (bind _gamehudref_3 (`self.gameHudRef`))
  ;[1 1 1] Move to current grid square center
  (`self.MoveToLocation` (`self.K2_GetActorLocation` (`self.myCurrentSpot`)) -1.0 false false false false)
  ;[1 1 1] Keep looping until stopped moving
  (if (<= (`self.GetDistanceTo` (`self.myCharRef`) (`self.myCurrentSpot`)) 50.0) :!label _label
    ;[1 1 1] Check if hero is in range, if so, then attack
    (bind _outactors (`GameplayStatics.GetAllActorsOfClass` "/Game/Main/Blueprints/Characters/BP_Hero_Character.BP_Hero_Character_C"))
    (bind _item (`KismetArrayLibrary.Array_Get` _outactors))
    (if (<= (`self.GetDistanceTo` (`self.myCharRef`) _item) 200.0)
      (set `/Game/Main/Blueprints/Widgets/BP_Game_HUD.attackerRef` (`self.myCharRef`) (`self.gameHudRef`))
      (set `/Game/Main/Blueprints/Widgets/BP_Game_HUD.victimRef` _item _gamehudref)
      (if (not (`self.hasAttacked`))
        (`/Game/Main/Blueprints/Widgets/BP_Game_HUD.Attack ` _gamehudref)
        (set `self.hasAttacked` true))
      (set `/Game/Main/Blueprints/Widgets/BP_Game_HUD.currentEnemyIndex` (+ (`/Game/Main/Blueprints/Widgets/BP_Game_HUD.currentEnemyIndex` _gamehudref_3) 1) _gamehudref_3)
      (`/Game/Main/Blueprints/Widgets/BP_Game_HUD.Perform Skeleton Actions` (`self.gameHudRef`))
      (else
        (set `/Game/Main/Blueprints/Widgets/BP_Game_HUD.currentEnemyIndex` (+ (`/Game/Main/Blueprints/Widgets/BP_Game_HUD.currentEnemyIndex` _gamehudref_2) 1) _gamehudref_2)
        (`/Game/Main/Blueprints/Widgets/BP_Game_HUD.Perform Skeleton Actions` (`self.gameHudRef`))))
    (else
      (`KismetSystemLibrary.Delay` 0.05)
      (goto _label))))

(fn `UserConstructionScript`)