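; BP_Skeleton_Character is a skeleton character that works with an AI controller and grid squares.
; On BeginPlay it casts its controller to BP_Skeleton_Controller and gives it a reference to itself.
; Overlap events mark any BP_Grid_Square it enters as occupied and clear that flag when it leaves.
; Tick and the construction script hold no logic.
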(event `self.ReceiveTick`
  (params (DeltaSeconds :type "Float (single-precision)"))
  (if true
    _))

(event `self.ReceiveBeginPlay`
  (bind _asaicontroller (cast `AIController` (`self.GetController`)))
  (bind _asbp_skeleton_controller (cast `/Game/Main/Blueprints/Characters/BP_Skeleton_Controller` _asaicontroller))
  (set `/Game/Main/Blueprints/Characters/BP_Skeleton_Controller.myCharRef` self _asbp_skeleton_controller))

(event `self.ReceiveActorBeginOverlap`
  (params (OtherActor :type "Actor Object Reference"))
  (if (`KismetMathLibrary.ClassIsChildOf` (`GameplayStatics.GetObjectClass` OtherActor) "/Game/Main/Blueprints/BP_Grid_Square.BP_Grid_Square_C")
    (bind _asbp_grid_square (cast `/Game/Main/Blueprints/BP_Grid_Square` OtherActor))
    (set `/Game/Main/Blueprints/BP_Grid_Square.isOccupied` true _asbp_grid_square)))

(event `self.ReceiveActorEndOverlap`
  (params (OtherActor :type "Actor Object Reference"))
  (if (`KismetMathLibrary.ClassIsChildOf` (`GameplayStatics.GetObjectClass` OtherActor) "/Game/Main/Blueprints/BP_Grid_Square.BP_Grid_Square_C")
    (bind _asbp_grid_square (cast `/Game/Main/Blueprints/BP_Grid_Square` OtherActor))
    (set `/Game/Main/Blueprints/BP_Grid_Square.isOccupied` false _asbp_grid_square)))

(fn `UserConstructionScript`)