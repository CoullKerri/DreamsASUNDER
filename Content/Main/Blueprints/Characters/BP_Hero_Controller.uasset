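; Controller for the player's hero in a turn-based grid tactics game, handling click-to-move, attack confirmation and turn hand-off.
; Clicking a grid square spawns a distance probe; a second click asks to confirm, and InitiateMove walks the PathPoints array.
; Skeleton clicks check range, then pass attacker and victim to the HUD.
; Tick ends the turn once moved and attacked, and maps WillAmount bands to damage.
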(event `self.ReceiveBeginPlay`
  (`|ExecutionSequence`
    (:`then_0`
      ;[1 1 1] Create Ref to the Hero Character
      (bind _returnvalue (`self.CastToPlayerController` (`GameplayStatics.GetPlayerController` 0)))
      (`self.EnableInput` _returnvalue)
      (bind (_foundactor _foundactorref) (`/Game/Main/Blueprints/BP_AI_Function_Library.CastToActorWithTag` "/Game/Main/Blueprints/Characters/BP_Hero_Character.BP_Hero_Character_C" (`self.myCharacterTag`)))
      (if _foundactor
        (set `self.myCharRef` _foundactorref)))
    (:`then_1`
      ;[1 1 1] Create Game Hud Ref
      (bind _foundwidgets (`WidgetBlueprintLibrary.GetAllWidgetsOfClass` "/Game/Main/Blueprints/Widgets/BP_Game_HUD.BP_Game_HUD_C"))
      (bind _asbp_game_hud (cast `/Game/Main/Blueprints/Widgets/BP_Game_HUD` (`KismetArrayLibrary.Array_Get` _foundwidgets)))
      (set `self.gameHudRef` _asbp_game_hud))
    (:`then_2`
      ;[1 1 1] Create reference to player camera
      (bind _outactors (`GameplayStatics.GetAllActorsOfClass` "/Game/Main/Blueprints/BP_Player_Camera.BP_Player_Camera_C"))
      (set `self.playerCamera` (`KismetArrayLibrary.Array_Get` _outactors)))
    (:`then_3`
      ;[1 1 1] Set variables to match data table values
      (bind _returnvalue_2 (`|GetDataTableRow` "/Game/Main/Blueprints/DataTables/Unit_Variable_Data.Unit_Variable_Data" "Player")
        (:`then`
          (bind (_hp _offense _defense _movement) (break `/Game/Main/Blueprints/DataTables/ST_Unit_Values` _returnvalue_2))
          (set `self.moveRange` (`KismetMathLibrary.FTrunc` _movement))
          (set `self.myHealth` (`KismetMathLibrary.FTrunc` _hp))
          (set `self.myDamage` (`KismetMathLibrary.FTrunc` _offense)))))))

(event `Disable Collision`
  ;[1 1 1] Disable the characters collision so it won't affect the nav mesh
  (bind _asbp_hero_character (cast `/Game/Main/Blueprints/Characters/BP_Hero_Character` (`self.myCharRef`)))
  (`PrimitiveComponent.SetCollisionEnabled` (`Character.CapsuleComponent` _asbp_hero_character) "NoCollision"))

(event `Enable Collision`
  ;[1 1 1] Re-enable the characters collision
  (bind _asbp_hero_character (cast `/Game/Main/Blueprints/Characters/BP_Hero_Character` (`self.myCharRef`)))
  (`PrimitiveComponent.SetCollisionEnabled` (`Character.CapsuleComponent` _asbp_hero_character) "QueryOnly"))

(event `Initiate Move`
  ;[1 1 1] Initiate the move
  (`self.DisableInput` (`GameplayStatics.GetPlayerController` 0))
  (`self.MoveToLocation` (`self.K2_GetActorLocation` (`KismetArrayLibrary.Array_Get` (`self.pathPoints`) (`self.currentPathIndex`))) -1.0 false true false false null false)
  (goto _label_2 :!via `Open`))

(event `RefreshPlayerActions`
  ;[1 1 1] Swap turns
  (goto _label :!via `Reset`))

(event `self.ReceiveTick`
  (params (DeltaSeconds :type "Float (single-precision)"))
  ;[1 1 1] Has the player performed both actions this turn
  (`|ExecutionSequence`
    (:`then_0`
      (if (and (`self.hasMoved`) (`self.hasAttacked`))
        ;[1 1 1] Swap turns
        (`/Engine/EditorBlueprintResources/StandardMacros.DoOnce` false :!label _label
          (:`Completed`
            (`/Game/Main/Blueprints/Widgets/BP_Game_HUD.Change Turn` (`self.gameHudRef`) "Enemy")))
        (else
          ;[1 1 1] TEMP - Setting health text render to face camera
          (bind _asbp_hero_character (cast `/Game/Main/Blueprints/Characters/BP_Hero_Character` (`self.myCharRef`)))
          (bind _healthtext (`/Game/Main/Blueprints/Characters/BP_Hero_Character.HealthText` _asbp_hero_character))
          (`SceneComponent.K2_SetWorldRotation` _healthtext (.rotation (`self.GetTransform` (`self.playerCamera`))) false false)
          (`SceneComponent.K2_AddLocalRotation` _healthtext (struct :`Pitch` 45.0 :`Yaw` 180.0) false false)
          ;[1 1 1] Set Health
          (`TextRenderComponent.K2_SetText` _healthtext (`KismetTextLibrary.Conv_IntToText` (`self.myHealth`)))
          ;[1 1 1] Determine the next path target along the array
          (`/Engine/EditorBlueprintResources/StandardMacros.Gate` true :!label _label_2
            (:`Exit`
              (if (<= (`self.GetDistanceTo` (`self.myCharRef`) (`KismetArrayLibrary.Array_Get` (`self.pathPoints`) (`self.currentPathIndex`))) 50.0)
                (set `self.currentPathIndex` (+ (`self.currentPathIndex`) 1))
                (if (`KismetSystemLibrary.IsValid` (`KismetArrayLibrary.Array_Get` (`self.pathPoints`) (`self.currentPathIndex`)))
                  (`self.Initiate Move`)
                  (else
                    (`|ExecutionSequence`
                      (:`then_0`
                        (goto _label_2 :!via `Close`))
                      (:`then_1`
                        (set `self.hasMoved` true)
                        (`self.EnableInput` (`GameplayStatics.GetPlayerController` 0))
                        (`self.ResetPath`)))))))))))
    (:`then_1`
      ;[1 1 1] Update will effects every so often
      (`KismetSystemLibrary.Delay` 0.2)
      (`self.Update Will Effects`))))

(event `Update Will Effects`
  (bind _willamount (`self.willAmount`))
  (bind _willamount_2 (`self.willAmount`))
  (bind _willamount_3 (`self.willAmount`))
  ;[1 1 1] Update the will meter and the will's effects based on its value in a range
  (if (and (>= _willamount 0.4) (<= _willamount 0.59))
    (set `self.myDamage` 10)
    (elif (and (>= _willamount_2 0.0) (<= _willamount_2 0.39))
      (set `self.myDamage` 5)
      (elif (and (>= _willamount_3 0.6) (<= _willamount_3 1.0))
        (set `self.myDamage` 15)))))

(event `InputAction|LeftMouseButton` :consume false
  (params (Key :type "Key Structure" :default "AnyKey"))
  (:`Pressed`
    (if (`KismetStringLibrary.EqualEqual_StrStr` (`/Game/Main/Blueprints/Widgets/BP_Game_HUD.Turn` (`self.gameHudRef`)) "Player")
      (if (== (`/Game/Main/Blueprints/Widgets/BP_Game_HUD.selectedActor` (`self.gameHudRef`)) (`self.myCharRef`))
        (bind (_was_found _clicked_actor_ref) (`self.Check For Enemy `))
        (if _was_found
          (if (`self.hasAttacked`)
            (`self.ResetSelection`)
            (else
              (set `self.clickedActorRef` _clicked_actor_ref)
              ;[1 1 1] Is character within range to attack
              (if (<= (`self.GetDistanceTo` (`self.myCharRef`) (`self.clickedActorRef`)) 200.0)
                ;[1 1 1] Offer Attack confirmation
                (`TextBlock.SetText` (`/Game/Main/Blueprints/Widgets/BP_Game_HUD.ActionText` (`self.gameHudRef`)) "Confirm Attack?")
                (`Widget.SetVisibility` (`/Game/Main/Blueprints/Widgets/BP_Game_HUD.ConfirmButton` (`self.gameHudRef`)) "Visible")
                (`Widget.SetVisibility` (`/Game/Main/Blueprints/Widgets/BP_Game_HUD.DeclineButton` (`self.gameHudRef`)) "Visible")
                (`Widget.SetVisibility` (`/Game/Main/Blueprints/Widgets/BP_Game_HUD.ActionPanel` (`self.gameHudRef`)) "Visible")
                ;[1 1 1] Send actor references to HUD
                (set `/Game/Main/Blueprints/Widgets/BP_Game_HUD.attackerRef` (`self.myCharRef`) (`self.gameHudRef`))
                (set `/Game/Main/Blueprints/Widgets/BP_Game_HUD.victimRef` (`self.clickedActorRef`) (`self.gameHudRef`))
                (else
                  ;[1 1 1] Display "Can't Attack due to distance" message
                  (`TextBlock.SetText` (`/Game/Main/Blueprints/Widgets/BP_Game_HUD.ActionText` (`self.gameHudRef`)) "Target is too Far - You must be adjacent in order to Attack")
                  (`Widget.SetVisibility` (`/Game/Main/Blueprints/Widgets/BP_Game_HUD.ActionPanel` (`self.gameHudRef`)) "Visible")
                  (`Widget.SetVisibility` (`/Game/Main/Blueprints/Widgets/BP_Game_HUD.ConfirmButton` (`self.gameHudRef`)) "Hidden")
                  (`Widget.SetVisibility` (`/Game/Main/Blueprints/Widgets/BP_Game_HUD.DeclineButton` (`self.gameHudRef`)) "Hidden")
                  (`KismetSystemLibrary.RetriggerableDelay` 2.0)
                  (if (`KismetTextLibrary.EqualEqual_TextText` (`TextBlock.GetText` (`/Game/Main/Blueprints/Widgets/BP_Game_HUD.ActionText` (`self.gameHudRef`))) "Target is too Far - You must be adjacent in order to Attack")
                    (`Widget.SetVisibility` (`/Game/Main/Blueprints/Widgets/BP_Game_HUD.ActionPanel` (`self.gameHudRef`)) "Hidden")
                    (`Widget.SetVisibility` (`/Game/Main/Blueprints/Widgets/BP_Game_HUD.ConfirmButton` (`self.gameHudRef`)) "Visible")
                    (`Widget.SetVisibility` (`/Game/Main/Blueprints/Widgets/BP_Game_HUD.DeclineButton` (`self.gameHudRef`)) "Visible"))))))
          (elif (not (`self.hasMoved`))
            ;[1 1 1] Check if the clicked target was a grid square before passing along its info
            (bind (_was_found_2 _actor_clicked) (`/Game/Main/Blueprints/BP_AI_Function_Library.RetrieveClickedTargetInfo` "/Game/Main/Blueprints/BP_Grid_Square.BP_Grid_Square_C"))
            (if _was_found_2
              (bind _output_get (set `self.clickedActorRef` _actor_clicked))
              (bind _asbp_grid_square (cast `/Game/Main/Blueprints/BP_Grid_Square` _output_get))
              (if (== (`PaperSpriteComponent.GetSprite` (`/Game/Main/Blueprints/BP_Grid_Square.Sprite` _asbp_grid_square)) "/Game/Main/Sprites/Grid_Box_Hover_Sprite.Grid_Box_Hover_Sprite")
                ;[1 1 1] Offer Move confirmation
                (`TextBlock.SetText` (`/Game/Main/Blueprints/Widgets/BP_Game_HUD.ActionText` (`self.gameHudRef`)) "Confirm Move?")
                (`Widget.SetVisibility` (`/Game/Main/Blueprints/Widgets/BP_Game_HUD.ConfirmButton` (`self.gameHudRef`)) "Visible")
                (`Widget.SetVisibility` (`/Game/Main/Blueprints/Widgets/BP_Game_HUD.DeclineButton` (`self.gameHudRef`)) "Visible")
                (`Widget.SetVisibility` (`/Game/Main/Blueprints/Widgets/BP_Game_HUD.ActionPanel` (`self.gameHudRef`)) "Visible")
                (else
                  (`Widget.SetVisibility` (`/Game/Main/Blueprints/Widgets/BP_Game_HUD.ActionPanel` (`self.gameHudRef`)) "Hidden")
                  (`PaperSpriteComponent.SetSprite` (`/Game/Main/Blueprints/BP_Grid_Square.Sprite` _asbp_grid_square) "/Game/Main/Sprites/Grid_Box_Hover_Sprite.Grid_Box_Hover_Sprite")
                  ;[1 1 1] Destroy the probe before making a new one
                  (bind _outactors (`GameplayStatics.GetAllActorsOfClass` "/Game/Main/Blueprints/DistanceProbe/BP_Distance_Probe.BP_Distance_Probe_C"))
                  (for _array_element _outactors
                    (`self.K2_DestroyActor` _array_element))
                  (`self.ResetPath`)
                  (`self.SendProbe` _output_get)))
              (else
                (`self.ResetSelection`)))))
        (else
          (`KismetSystemLibrary.PrintString` "Hero not selected"))))))

(event `Key|P`
  (params (Key :type "Key Structure" :default "AnyKey"))
  ;[1 1 1] Debug for changing turns
  (:`Pressed`
    (`/Game/Main/Blueprints/Widgets/BP_Game_HUD.Change Turn` (`self.gameHudRef`) "Enemy")))

(event `ResetSelection`
  ;[1 1 1] Called when the player clicks outside of playable space while this unit is selected
  (bind _asbp_hero_character (cast `/Game/Main/Blueprints/Characters/BP_Hero_Character` (`self.myCharRef`)))
  (`PrimitiveComponent.SetMaterial` (`Character.Mesh` _asbp_hero_character) 0 "/Game/Mannequin/Character/Materials/M_UE4Man_Body.M_UE4Man_Body")
  (set `/Game/Main/Blueprints/Widgets/BP_Game_HUD.selectedActor` null (`self.gameHudRef`)))

(fn `Check For Enemy `
  (returns (`Was Found` :type Boolean) (`Clicked Actor Ref` :type "Actor Object Reference"))
  ;[1 1 1] Check for Skeleton
  (bind (_was_found _actor_clicked) (`/Game/Main/Blueprints/BP_AI_Function_Library.RetrieveClickedTargetInfo` "/Game/Main/Blueprints/Characters/BP_Skeleton_Character.BP_Skeleton_Character_C"))
  (if _was_found
    (return true _actor_clicked)
    (else
      (return false null))))

(fn `ResetPath`
  ;[1 1 1] Resets all grid square to the default sprite
  (bind _outactors (`GameplayStatics.GetAllActorsOfClass` "/Game/Main/Blueprints/BP_Grid_Square.BP_Grid_Square_C"))
  (for _array_element _outactors
    (`PaperSpriteComponent.SetSprite` (`/Game/Main/Blueprints/BP_Grid_Square.Sprite` _array_element) "/Game/Main/Sprites/Grid_Box_Normal_Sprite.Grid_Box_Normal_Sprite")
    ;[1 1 1] Clears Path Array
    (`KismetArrayLibrary.Array_Clear` (`self.pathPoints`))
    (set `self.currentPathIndex` 0)
    ;[1 1 1] Destroys the probe
    (bind _outactors_2 (`GameplayStatics.GetAllActorsOfClass` "/Game/Main/Blueprints/DistanceProbe/BP_Distance_Probe.BP_Distance_Probe_C"))
    (for _array_element_2 _outactors_2
      (`self.K2_DestroyActor` _array_element_2))
    ;[1 1 1] Hides the action panel
    (`Widget.SetVisibility` (`/Game/Main/Blueprints/Widgets/BP_Game_HUD.ActionPanel` (`self.gameHudRef`)) "Hidden")))

(fn `SendProbe`
  (params (ClickedActorRef :type "Actor Object Reference"))
  (bind _returnvalue (`|SpawnActorFromClass` "/Game/Main/Blueprints/DistanceProbe/BP_Distance_Probe.BP_Distance_Probe_C" (`self.GetTransform` (`self.myCharRef`)) "AlwaysSpawn" "OverrideRootScale"))
  (set `/Game/Main/Blueprints/DistanceProbe/BP_Distance_Probe.myTargetToPassOn` ClickedActorRef _returnvalue)
  (set `/Game/Main/Blueprints/DistanceProbe/BP_Distance_Probe.myOwnerPassOn` self _returnvalue)
  (set `/Game/Main/Blueprints/DistanceProbe/BP_Distance_Probe.moveRange` (`self.moveRange`) _returnvalue)
  (`/Game/Main/Blueprints/DistanceProbe/BP_Distance_Probe.MoveToTarget` _returnvalue))

(fn `UserConstructionScript`)