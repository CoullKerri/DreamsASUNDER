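; BP_Distance_Probe is an AI-driven probe that travels toward a target to record the grid-square path for a unit's move.
; MoveToTarget hands target and owner to BP_Distance_Probe_Controller, while overlaps highlight and store each crossed grid square.
; On nearing the target or hitting MoveRange, it copies the squares into the owning Hero controller's PathPoints and destroys itself.
; Touching a skeleton destroys it without reporting; the Revenant branch is empty.
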(event `self.ReceiveDestroyed`
  (`KismetSystemLibrary.PrintString` "reached target"))

(event `self.ReceiveTick`
  (params (DeltaSeconds :type "Float (single-precision)"))
  ;[1 1 1] If the player reaches the target, destroy the probe and relay path back to player
  (if (<= (`self.GetDistanceTo` (`self.myTargetToPassOn`)) 50.0)
    (`self.SendArrayBackToOwner`)
    (`self.K2_DestroyActor`)))

(event `self.ReceiveBeginPlay`)

(event `self.ReceiveActorBeginOverlap`
  (params (OtherActor :type "Actor Object Reference"))
  (if (`KismetMathLibrary.ClassIsChildOf` (`GameplayStatics.GetObjectClass` OtherActor) "/Game/Main/Blueprints/Characters/BP_Skeleton_Character.BP_Skeleton_Character_C")
    (`self.K2_DestroyActor`)
    (else
      ;[1 1 1] On each grid square collision, set it as highlighted
      (if (`KismetMathLibrary.ClassIsChildOf` (`GameplayStatics.GetObjectClass` OtherActor) "/Game/Main/Blueprints/BP_Grid_Square.BP_Grid_Square_C")
        (bind _asbp_grid_square (cast `/Game/Main/Blueprints/BP_Grid_Square` OtherActor))
        (`PaperSpriteComponent.SetSprite` (`/Game/Main/Blueprints/BP_Grid_Square.Sprite` _asbp_grid_square) "/Game/Main/Sprites/Grid_Box_Hover_Sprite.Grid_Box_Hover_Sprite")
        (bind _returnvalue (`KismetArrayLibrary.Array_Add` (`self.crossedGridSquares`) OtherActor))
        (if (== _returnvalue (`self.moveRange`))
          (`self.SendArrayBackToOwner`)
          (`self.K2_DestroyActor`))))))

(event `self.Cube.OnComponentBeginOverlap`
  (params (OtherActor :type "Actor Object Reference") (OtherComp :type "PrimitiveComponent Object Reference") (OtherBodyIndex :type Integer) (bFromSweep :type Boolean) (SweepResult :type "HitResult Structure (by ref)")))

(event `MoveToTarget`
  ;[1 1 1] Send off action info to the controller (To Cause the Move)
  (bind _asaicontroller (cast `AIController` (`self.GetController`)))
  (bind _asbp_distance_probe_controller (cast `/Game/Main/Blueprints/DistanceProbe/BP_Distance_Probe_Controller` _asaicontroller))
  (set `/Game/Main/Blueprints/DistanceProbe/BP_Distance_Probe_Controller.myTarget` (`self.myTargetToPassOn`) _asbp_distance_probe_controller)
  (set `/Game/Main/Blueprints/DistanceProbe/BP_Distance_Probe_Controller.myOwner` (`self.myOwnerPassOn`) _asbp_distance_probe_controller)
  (`/Game/Main/Blueprints/DistanceProbe/BP_Distance_Probe_Controller.MoveToTarget` _asbp_distance_probe_controller))

(fn `SendArrayBackToOwner`
  (if (`KismetMathLibrary.ClassIsChildOf` (`GameplayStatics.GetObjectClass` (`self.myOwnerPassOn`)) (`.Hero_16_3671E1EF4B519DE7894DCFB6E352041E` (break `/Game/Main/Blueprints/DistanceProbe/ST_Unit_Types` (make `/Game/Main/Blueprints/DistanceProbe/ST_Unit_Types` "/Game/Main/Blueprints/Characters/BP_Hero_Controller.BP_Hero_Controller_C"))))
    (bind _asbp_hero_controller (cast `/Game/Main/Blueprints/Characters/BP_Hero_Controller` (`self.myOwnerPassOn`)))
    (set `/Game/Main/Blueprints/Characters/BP_Hero_Controller.pathPoints` (`self.crossedGridSquares`) _asbp_hero_controller)
    (elif false
      _)))

(fn `UserConstructionScript`)