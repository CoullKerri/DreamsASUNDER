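; Grid square actor that can act as a pawn spawn point.
; On BeginPlay, a square flagged as a spawn point spawns its configured pawn with AI slightly above itself, ignoring collision, then stores a hero character reference found by the "Hero" tag.
; Cursor-over events are empty, and the hover/normal sprite swaps are disconnected, so no highlight runs.
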(event `self.ReceiveActorBeginCursorOver`)

(event `self.ReceiveActorEndCursorOver`)

(event `self.ReceiveActorBeginOverlap`
  (params (OtherActor :type "Actor Object Reference")))

(event `self.ReceiveTick`
  (params (DeltaSeconds :type "Float (single-precision)")))

(event `self.ReceiveBeginPlay`
  (if (`self.isSpawnPoint`)
    (`AIBlueprintHelperLibrary.SpawnAIFromClass` (`self.spawnedPawn`) null (+ (.location (`self.GetTransform`)) (0.0 0.0 8.0)) (struct) true)
    (bind (_foundactor _foundactorref) (`/Game/Main/Blueprints/BP_AI_Function_Library.CastToActorWithTag` "/Game/Main/Blueprints/BP_Hero_Character.BP_Hero_Character_C" "Hero"))
    (if _foundactor
      (set `self.charRef` _foundactorref))))

(fn `UserConstructionScript`)